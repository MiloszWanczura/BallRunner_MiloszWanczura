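; BP_Crystal is a collectable crystal that flies into the player and vanishes when its sphere overlap passes the IsPlayer check.
; On pickup it caches its location, scale and light intensity, then plays a timeline with separate tracks for movement, shrinking and light fade.
; Movement lerps toward the pawn's current location each update, so it follows a moving player, and the actor is destroyed when the timeline finishes.
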(event `self.Sphere.OnComponentBeginOverlap`
  (params (OverlappedComponent :type "PrimitiveComponent Object Reference") (OtherActor :type "Actor Object Reference") (OtherComp :type "PrimitiveComponent Object Reference") (OtherBodyIndex :type Integer) (bFromSweep :type Boolean) (SweepResult :type "HitResult Structure (by ref)"))
  (`self.IsPlayer` 0.0
    (:`IsPlayer`
      (`self.F_Info`)
      (bind (_direction _newtrack_0 _scale _lighting) (`Timeline|Tl_BlendAlpha` :`NewTime` 0.7)
        (:`Update`
          (`self.F_CrystalLocation` _newtrack_0)
          (`self.F_CrystalScale` _scale)
          (`self.F_CrystalLight` _lighting))
        (:`Finished`
          (`self.K2_DestroyActor`))))))

(fn `F_CrystalLight`
  (params (Alpha :type "Float (double-precision)"))
  (`LightComponent.SetIntensity` (`self.PointLight`) (`KismetMathLibrary.Lerp` (`self.CrystalLight`) 0.0 Alpha)))

(fn `F_CrystalLocation`
  (params (Alpha :type "Float (double-precision)"))
  (`self.K2_SetActorLocation` (`KismetMathLibrary.VLerp` (`self.LerpStartLocation`) (`self.K2_GetActorLocation` (`GameplayStatics.GetPlayerPawn` 0)) Alpha)))

(fn `F_CrystalScale`
  (params (Alpha :type "Float (double-precision)"))
  (`self.SetActorScale3D` (`KismetMathLibrary.VLerp` (`self.CrystalScale`) (0.0 0.0 0.0) Alpha)))

(fn `F_Info`
  (set `self.LerpStartLocation` (`self.K2_GetActorLocation`))
  (set `self.BallLocation` (`self.K2_GetActorLocation` (`GameplayStatics.GetPlayerPawn` 0)))
  (set `self.CrystalLight` (`LightComponentBase.Intensity` (`self.PointLight`)))
  (set `self.CrystalScale` (`self.GetActorScale3D`)))

(fn `UserConstructionScript`)