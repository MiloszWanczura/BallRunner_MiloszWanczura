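; BP_WinVolume is a level-exit volume that completes the level when the player pawn overlaps it and no crystals remain.
; On overlap it counts remaining BP_Crystal actors, printing a Polish warning if any are left or a congratulation otherwise.
; Completion finds the current level in the ordered LevelNames array and opens the next entry, or quits the game on the last one.
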(event `self.ReceiveActorBeginOverlap`
  (params (OtherActor :type "Actor Object Reference"))
  (`self.IsPlayer` OtherActor)
  (bind _output_get (set `self.check any crystals left` (`self.CheckanyCrystals`)))
  (if _output_get
    (`KismetSystemLibrary.PrintText` "nie zebrałes wszystkich krysztalow")
    (else
      (`KismetSystemLibrary.PrintText` "brawo")
      (`self.Complete level`))))

(fn `CheckanyCrystals`
  (returns (Info :type Boolean))
  (bind _outactors (`GameplayStatics.GetAllActorsOfClass` "/Game/Blueprints/Actors/Collectables/BP_Crystal.BP_Crystal_C"))
  (return (`KismetMathLibrary.Conv_IntToBool` (`KismetArrayLibrary.Array_Length` _outactors))))

(fn `Complete level`
  (if (`self.Is Final`)
    (`KismetSystemLibrary.QuitGame` null "Quit")
    (else
      (`self.LoadNextLevel`))))

(fn `GetCurrentLvlName`
  (returns (ReturnValue :type Integer))
  (bind _returnvalue (`GameplayStatics.GetCurrentLevelName` true))
  (return (`KismetArrayLibrary.Array_Find` (`self.LevelNames`) (`KismetStringLibrary.Conv_StringToName` _returnvalue))))

(fn `Is Final`
  (returns (NewParam :type Boolean))
  (return (== (`KismetArrayLibrary.Array_LastIndex` (`self.LevelNames`)) (`self.GetCurrentLvlName`))))

(fn `LoadNextLevel`
  (`GameplayStatics.OpenLevel` (`|GetArrayItem` (`self.LevelNames`) (+ (`self.GetCurrentLvlName`) 1))))

(fn `UserConstructionScript`)