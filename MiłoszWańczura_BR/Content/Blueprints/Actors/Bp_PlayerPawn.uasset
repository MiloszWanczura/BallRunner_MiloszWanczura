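; Player pawn that moves by applying torque to its static mesh and restarts the level when it takes any damage.
; Forward/back and left/right axes share one torque call, feeding the axis value into both X and Y torque.
; Damage runs the Reset macro, which prints a message, fades the camera to black and reopens the current level after a delay.
; RameraMenagment sets spring arm rotation and scale but is not called here.
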(event `self.ReceiveAnyDamage`
  (params (Damage :type "Float (single-precision)") (DamageType :type "DamageType Object Reference") (InstigatedBy :type "Controller Object Reference") (DamageCauser :type "Actor Object Reference"))
  (`self.Reset`))

(event `InputAxis|Przód/Tył`
  (params (AxisValue :type "Float (single-precision)"))
  (`PrimitiveComponent.AddTorqueInRadians` (`self.StaticMesh`) (`KismetMathLibrary.MakeVector` (stale `InputAxis|Lewo/Prawo` AxisValue) AxisValue) "None" (`self.TS`) :!label _label))

(event `InputAxis|Lewo/Prawo`
  (params (AxisValue :type "Float (single-precision)"))
  (goto _label))

(fn `RameraMenagment`
  (`SceneComponent.K2_SetRelativeRotation` (`self.SpringArm`) (struct :`Pitch` -65.0) false false)
  (`SceneComponent.SetRelativeScale3D` (`self.SpringArm`) (30.0 30.0 30.0))
  (return))

(fn `UserConstructionScript`)