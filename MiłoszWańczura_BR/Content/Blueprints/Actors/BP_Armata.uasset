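; BP_Armata is a cannon actor that fires projectiles automatically in an endless loop from BeginPlay.
; Each cycle waits for the fire-rate delay, then spawns a Bullet using the Arrow component's world location and rotation and a configurable scale.
; The Armata timeline then animates the Cannon component's relative Y location as barrel movement, and its Finished output restarts the cycle.
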(event `self.ReceiveBeginPlay`
  (`KismetSystemLibrary.Delay` (`self.FIrerate`) :!label _label)
  (bind (_returnvalue _returnvalue2 _returnvalue3) (`self.SpawnProjectile`))
  (`|SpawnActorFromClass` "/Game/Blueprints/Actors/Projectiles/Bullet.Bullet_C" (`KismetMathLibrary.MakeTransform` _returnvalue2 _returnvalue _returnvalue3) "Undefined" "OverrideRootScale" null null)
  (bind (_direction _cannonbarrellocation) (`Timeline|Armata` :!via `PlayFromStart`)
    (:`Update`
      (`SceneComponent.K2_SetRelativeLocation` (`self.Cannon`) (`KismetMathLibrary.MakeVector` 0.0 _cannonbarrellocation) false false))
    (:`Finished`
      (goto _label))))

(fn `SpawnProjectile`
  (returns (ReturnValue :type "Rotator Structure") (ReturnValue2 :type "Vector Structure") (ReturnValue3 :type "Vector Structure"))
  (return (`SceneComponent.K2_GetComponentRotation` (`self.Arrow`)) (`SceneComponent.K2_GetComponentLocation` (`self.Arrow`)) (`KismetMathLibrary.Conv_DoubleToVector` (`self.Scale`))))

(fn `UserConstructionScript`)